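; Game instance that manages menus, multiplayer sessions and persistent score and record data.
; Menu events create and cache widgets, while lobby creation advertises name, map, mode and LAN through Advanced Sessions, then opens a listen server.
; Back, server menu and join events destroy any existing session first.
; Save functions use one slot, but Init's load-or-create check is disconnected; Init caps FPS, and another event resets Steam achievements.
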(event `self.ReceiveInit`
  ;[0.05524 0.1216 1] Система сохранений
  (`KismetSystemLibrary.PrintString` "Сохранение отключено")
  (`KismetSystemLibrary.ExecuteConsoleCommand` "t.MaxFPS 60" null))

(event `Achievements_NULL`
  (bind _returnvalue (`GameplayStatics.GetPlayerController` 0))
  ;[0 0 0] Обнуление ачивки СТИМ
  (`AchievementQueryCallbackProxy.CacheAchievements` _returnvalue
    (:`OnSuccess`
      (`AchievementWriteCallbackProxy.WriteAchievementProgress` _returnvalue "ACH_WIN_ONE_GAME" 0.0
        (:`then`
          (`AchievementWriteCallbackProxy.WriteAchievementProgress` _returnvalue "ACH_WIN_100_GAMES" 0.0
            (:`then`
              (`AchievementWriteCallbackProxy.WriteAchievementProgress` _returnvalue "ACH_TRAVEL_FAR_ACCUM" 0.0
                (:`then`
                  (`AchievementWriteCallbackProxy.WriteAchievementProgress` _returnvalue "ACH_TRAVEL_FAR_SINGLE" 0.0))))))))))

(event `MainMenu`
  (bind _returnvalue (`GameplayStatics.GetPlayerController` 0))
  ;[0.5647 0 0.7379] Создание главного меню и логика кнопки назад
  (`/Engine/EditorBlueprintResources/StandardMacros.IsValid` (`self.MenuMain`) :!label _label
    (:`Is Valid`
      _)
    (:`Is Not Valid`
      (bind _returnvalue_2 (`|CreateWidget` "/Game/MyGame/UI/WBP_MENU.WBP_MENU_C" (`GameplayStatics.GetPlayerController` 0)))
      (bind _output_get (set `self.MenuMain` _returnvalue_2))))
  (`Widget.SetVisibility` _output_get "Visible")
  (`UserWidget.AddToViewport` _output_get 0)
  (set `PlayerController.bShowMouseCursor` true _returnvalue)
  (`WidgetBlueprintLibrary.SetInputMode_UIOnlyEx` _returnvalue (`self.MenuMain`) "LockOnCapture"))

(event `Back`
  ;[0.5647 0 0.7379] Создание главного меню и логика кнопки назад
  (`DestroySessionCallbackProxy.DestroySession` (`GameplayStatics.GetPlayerController` 0)
    (:`OnSuccess`
      _)
    (:`OnFailure`
      _))
  (`KismetSystemLibrary.Delay` 0.2)
  (`WidgetLayoutLibrary.RemoveAllWidgets`)
  (goto _label))

(event `ServerMenu`
  ;[0.5647 0 0.7373] Создание меню создание сервера
  (`DestroySessionCallbackProxy.DestroySession` (`GameplayStatics.GetPlayerController` 0)
    (:`then`
      (`/Engine/EditorBlueprintResources/StandardMacros.IsValid` (`self.MenuServer`)
        (:`Is Valid`
          _)
        (:`Is Not Valid`
          (bind _returnvalue (`|CreateWidget` "/Game/MyGame/UI/WBP_Menu_Server.WBP_Menu_Server_C" (`GameplayStatics.GetPlayerController` 0)))
          (bind _output_get (set `self.MenuServer` _returnvalue))))
      (`UserWidget.AddToViewport` _output_get 0))))

(event `JoinGame`
  (params (SessionToJoin :type "BlueprintSessionResult Structure"))
  (bind _returnvalue (`GameplayStatics.GetPlayerController` 0))
  ;[0.5647 0 0.7373] Присоеденится к сессии
  (`WidgetLayoutLibrary.RemoveAllWidgets`)
  (`DestroySessionCallbackProxy.DestroySession` _returnvalue
    (:`OnSuccess`
      _)
    (:`OnFailure`
      _))
  (bind _returnvalue_2 (`|CreateWidget` "/Game/MyGame/UI/PreConstract/Wpre_Loading.Wpre_Loading_C" _returnvalue))
  (`UserWidget.AddToViewport` _returnvalue_2 0)
  (`JoinSessionCallbackProxy.JoinSession` _returnvalue SessionToJoin
    (:`OnFailure`
      (`KismetSystemLibrary.PrintString` "Session failed"))))

(event `CreateLobby`
  (params (ServerName :type String) (ServerMap :type String) (ServerMode :type String) (ServerSlots :type Integer) (`ServerMethod_Lan?` :type Boolean))
  ;[0.5647 0 0.7373] Начало игры
  (set `self.ServerName` ServerName)
  (set `self.ServerMap` ServerMap)
  (set `self.ServerMode` ServerMode)
  (set `self.ServerSlots` ServerSlots)
  (set `self.ServerMethod_Lan?` `ServerMethod_Lan?`)
  (`CreateSessionCallbackProxyAdvanced.CreateAdvancedSession` (`|MakeArray` (`AdvancedSessionsLibrary.MakeLiteralSessionPropertyString` "NAME" (`self.ServerName`)) (`AdvancedSessionsLibrary.MakeLiteralSessionPropertyString` "MAP" (`self.ServerMap`)) (`AdvancedSessionsLibrary.MakeLiteralSessionPropertyString` "MODE" (`self.ServerMode`)) (`AdvancedSessionsLibrary.MakeLiteralSessionPropertyBool` "LAN" (`self.ServerMethod_Lan?`))) (`GameplayStatics.GetPlayerController` 0) (`self.ServerSlots`) 0 (`self.ServerMethod_Lan?`)
    (:`OnSuccess`
      (`GameplayStatics.OpenLevel` (`KismetStringLibrary.Conv_StringToName` (`self.ServerMap`)) true "listen"))
    (:`OnFailure`
      (`KismetSystemLibrary.PrintString` "Start Failure"))))

(fn `DeleteSave`
  (`GameplayStatics.DeleteGameInSlot` "1"))

(fn `LoadGame`
  ;[1 1 1] Загрузка сейва
  (bind _returnvalue (`GameplayStatics.LoadGameFromSlot` "1"))
  (bind _asbp_save_game (cast `/Game/MyGame/Blueprints/SaveSystem/BP_SaveGame` _returnvalue))
  (`|ExecutionSequence`
    (:`then_0`
      (bind (_score _recordscore _playername _recordname) (break `/Game/MyGame/Blueprints/SaveSystem/S_SaveGameStructure` (`/Game/MyGame/Blueprints/SaveSystem/BP_SaveGame.SaveGameStructure` _asbp_save_game)))
      (set `self.Score` _score))
    (:`then_1`
      (set `self.RecordScore` _recordscore))
    (:`then_2`
      (set `self.PlayerName` _playername))
    (:`then_3`
      (set `self.RecordName` _recordname))))

(fn `SaveGame`
  ;[1 1 1] Создание сейва
  (bind _returnvalue (`GameplayStatics.CreateSaveGameObject` "/Game/MyGame/Blueprints/SaveSystem/BP_SaveGame.BP_SaveGame_C"))
  (set `/Game/MyGame/Blueprints/SaveSystem/BP_SaveGame.SaveGameStructure` (make `/Game/MyGame/Blueprints/SaveSystem/S_SaveGameStructure` (`self.Score`) (`self.RecordScore`) (`self.PlayerName`) (`self.RecordName`)) _returnvalue)
  (`GameplayStatics.SaveGameToSlot` _returnvalue "1")
  (`KismetSystemLibrary.PrintString` "Сохранение создано" true true (struct :`G` 0.66 :`B` 1.0 :`A` 1.0) 10.0))

(fn `SaveItems`
  (params (Cheese :type Integer))
  (set `self.Score` (+ Cheese (`self.Score`))))

(fn `SaveRecord`
  (params (CurrentScore :type Integer))
  (if (> CurrentScore (`self.RecordScore`))
    (`|ExecutionSequence`
      (:`then_0`
        (set `self.RecordName` (`self.PlayerName`)))
      (:`then_1`
        (set `self.RecordScore` (`local.CurrentScore`))))))